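; Frog NPC Blueprint with a simple enum-driven behavior sketch for wandering, seeking food and following a target.
; The construction script starts it Idle and Homeless; dwelling and hunger are meant to select the state, which drives AI MoveTo.
; That logic and the hunger timer are disconnected from the empty Tick, so they never run.
; FindClosestFood moves to whichever Frog_Interactable_BP GetActorOfClass returns, without comparing distance.
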(event `self.ReceiveTick`
  (params (DeltaSeconds :type "Float (single-precision)")))

(event `FindClosestFood`
  ;[1 1 1] Find Closest food
  (bind _returnvalue (`GameplayStatics.GetActorOfClass` "/Game/Enviorment/Frog_Interactable_BP.Frog_Interactable_BP_C"))
  (`|AIMoveTo` self (0.0 0.0 0.0) _returnvalue))

(fn `UserConstructionScript`
  (set `self.CurrentState` "NewEnumerator0")
  (set `self.CurrentDwelling` "NewEnumerator0"))